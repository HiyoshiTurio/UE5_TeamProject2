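; Player character that moves, looks, jumps and fires bullets.
; Input Action events add movement along the actor's forward and right vectors, drive controller pitch and yaw, and call Jump.
; Shooting spawns BP_Bullet at the Cylinder component's location (socket "None") plus FireSocketOffset rotated by actor rotation.
; The bullet takes its facing from actor rotation, not control rotation.
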(event Input|EnhancedActionEvents|EnhancedInputActionIA_Moveforward
  (params (ActionValue :type Float%20%28double-precision%29) (ElapsedSeconds :type Float%20%28double-precision%29) (TriggeredSeconds :type Float%20%28double-precision%29) (InputAction :type Input%20Action%20Object%20Reference :default "/Game/ProjectContent/Player/IA_Moveforward.IA_Moveforward"))
  (Pawn|Input|AddMovementInput (Transformation|GetActorForwardVector) ActionValue false))

(event Input|EnhancedActionEvents|EnhancedInputActionIA_MoveRight
  (params (ActionValue :type Float%20%28double-precision%29) (ElapsedSeconds :type Float%20%28double-precision%29) (TriggeredSeconds :type Float%20%28double-precision%29) (InputAction :type Input%20Action%20Object%20Reference :default "/Game/ProjectContent/Player/IA_MoveRight.IA_MoveRight"))
  (Pawn|Input|AddMovementInput (Transformation|GetActorRightVector) ActionValue false))

(event Input|EnhancedActionEvents|EnhancedInputActionIA_Look
  (params (ActionValue :type Float%20%28double-precision%29) (ElapsedSeconds :type Float%20%28double-precision%29) (TriggeredSeconds :type Float%20%28double-precision%29) (InputAction :type Input%20Action%20Object%20Reference :default "/Game/ProjectContent/Player/IA_Look.IA_Look"))
  (Pawn|Input|AddControllerPitchInput ActionValue))

(event Input|EnhancedActionEvents|EnhancedInputActionIA_Jump
  (params (ActionValue :type Boolean) (ElapsedSeconds :type Float%20%28double-precision%29) (TriggeredSeconds :type Float%20%28double-precision%29) (InputAction :type Input%20Action%20Object%20Reference :default "/Game/ProjectContent/Player/IA_Jump.IA_Jump"))
  (Character|Jump))

(event Input|EnhancedActionEvents|EnhancedInputActionIA_Turn
  (params (ActionValue :type Float%20%28double-precision%29) (ElapsedSeconds :type Float%20%28double-precision%29) (TriggeredSeconds :type Float%20%28double-precision%29) (InputAction :type Input%20Action%20Object%20Reference :default "/Game/ProjectContent/Player/IA_Turn.IA_Turn"))
  (Pawn|Input|AddControllerYawInput ActionValue))

(event Input|EnhancedActionEvents|EnhancedInputActionIA_Shoot
  (params (ActionValue :type Boolean) (ElapsedSeconds :type Float%20%28double-precision%29) (TriggeredSeconds :type Float%20%28double-precision%29) (InputAction :type Input%20Action%20Object%20Reference :default "/Game/ProjectContent/Player/IA_Shoot.IA_Shoot"))
  (bind _returnvalue (Transformation|GetActorRotation))
  (Game|SpawnActorfromClass "/Game/ProjectContent/Pistol/BP_Bullet.BP_Bullet_C" (Math|Transform|MakeTransform (+ (Transformation|GetSocketLocation (Variables|Default|GetCylinder) "None") (Math|Vector|RotateVector (Variables|Default|GetFireSocketOffset) _returnvalue)) _returnvalue) "Undefined" "MultiplyWithRoot" 0 0))

(event EventBeginPlay)

(event Collision|EventActorBeginOverlap
  (params (OtherActor :type Actor%20Object%20Reference)))

(event EventTick
  (params (DeltaSeconds :type Float%20%28single-precision%29)))

(fn ConstructionScript)